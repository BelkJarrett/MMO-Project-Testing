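; Kunai projectile for the Ninja character's weapons, setting its scale and lifespan on spawn.
; Kunai overlaps with damageable actors other than the instigator apply engine damage credited to the instigator's controller, then destroy the projectile.
; A separate DamageBox overlap subtracts fixed health directly from NewAIBase enemies, without the instigator check.
; OnBlockingImpact sets lifespan to zero, which cancels timed expiry, but nothing in these graphs calls it.
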(event `self.Kunai.OnComponentBeginOverlap`
  (params (OverlappedComponent :type "PrimitiveComponent Object Reference") (OtherActor :type "Actor Object Reference") (OtherComp :type "PrimitiveComponent Object Reference") (OtherBodyIndex :type Integer) (bFromSweep :type Boolean) (SweepResult :type "HitResult Structure (by ref)"))
  (if (`Actor.bCanBeDamaged` OtherActor)
    (if (not (== (`self.GetInstigator`) OtherActor))
      (`self.OnImpact` OtherActor SweepResult))))

(event `self.DamageBox.OnComponentBeginOverlap`
  (params (OverlappedComponent :type "PrimitiveComponent Object Reference") (OtherActor :type "Actor Object Reference") (OtherComp :type "PrimitiveComponent Object Reference") (OtherBodyIndex :type Integer) (bFromSweep :type Boolean) (SweepResult :type "HitResult Structure (by ref)"))
  (bind _asnew_aibase (cast `/Game/Characters/AI_Characters/AITesting/NewAIBase` OtherActor))
  (`/Game/Characters/AI_Characters/AITesting/NewAIBase.EditAIHealth` _asnew_aibase -10.0 _asnew_aibase))

(event `self.ReceiveBeginPlay`
  (`self.SetActorScale3D` (`self.Projectile Scale`))
  (`self.SetLifeSpan` (`self.Projectile Life`)))

(fn `OnBlockingImpact`
  (`self.SetLifeSpan` 0.0))

(fn `OnImpact`
  (params (DamageActor :type "Actor Object Reference") (`Hit Info` :type "HitResult Structure"))
  (`GameplayStatics.ApplyDamage` DamageActor (`self.Damage`) (`self.GetInstigatorController`) self)
  (`self.K2_DestroyActor`))

(fn `UserConstructionScript`)