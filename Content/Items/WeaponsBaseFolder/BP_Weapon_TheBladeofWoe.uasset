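; Blade of Woe weapon that the player can pick up, carry on the sheath socket and use to damage AI.
; Pickup swaps out any equipped weapon, leaving it at this blade's spot, then registers the blade and its weapon type on the BaseFunction player character.
; DamageBox overlaps apply fixed damage through NewAIBase's EditAIHealth.
; AttackReady and AttackNotReady toggle an Attacking flag, which the overlap handler does not check.
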(event `/Game/Items/WeaponsBaseFolder/WeaponInteract.PickUpWeapon`
  (bind _defaultsceneroot (`self.DefaultSceneRoot`))
  (bind _asbase_function (cast `/Game/Characters/BaseFunction` (`GameplayStatics.GetPlayerCharacter` 0) :!pure true))
  (bind _equippedweapon (`/Game/Characters/BaseFunction.EquippedWeapon` (cast `/Game/Characters/BaseFunction` (`GameplayStatics.GetPlayerCharacter` 0) :!pure true)))
  ;[1 1 1] Weapon PickUp
  (`/Engine/EditorBlueprintResources/StandardMacros.IsValid` _equippedweapon
    (:`Is Valid`
      (`self.K2_DetachFromActor` _equippedweapon "KeepRelative" "KeepRelative" "KeepRelative")
      (`self.K2_SetActorLocationAndRotation` _equippedweapon (`SceneComponent.K2_GetComponentLocation` _defaultsceneroot) (`SceneComponent.K2_GetComponentRotation` _defaultsceneroot) false false))
    (:`Is Not Valid`
      _))
  (set `/Game/Characters/BaseFunction.EquippedWeapon` self _asbase_function)
  (set `/Game/Characters/BaseFunction.WeaponType` 0 _asbase_function)
  (`self.K2_AttachToComponent` (`Character.Mesh` _asbase_function) "Weapon_Sheath" "SnapToTarget" "SnapToTarget" "SnapToTarget"))

(event `/Game/Items/WeaponsBaseFolder/WeaponInteract.AttackReady`
  (set `self.Attacking?` true))

(event `/Game/Items/WeaponsBaseFolder/WeaponInteract.AttackNotReady`
  (set `self.Attacking?` false))

(event `self.DamageBox.OnComponentBeginOverlap`
  (params (OverlappedComponent :type "PrimitiveComponent Object Reference") (OtherActor :type "Actor Object Reference") (OtherComp :type "PrimitiveComponent Object Reference") (OtherBodyIndex :type Integer) (bFromSweep :type Boolean) (SweepResult :type "HitResult Structure (by ref)"))
  (bind _asnew_aibase (cast `/Game/Characters/AI_Characters/AITesting/NewAIBase` OtherActor))
  (`/Game/Characters/AI_Characters/AITesting/NewAIBase.EditAIHealth` _asnew_aibase -8.0 _asnew_aibase))

(fn `UserConstructionScript`
  (`parent.UserConstructionScript`))