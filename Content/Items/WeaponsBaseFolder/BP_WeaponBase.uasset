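; BP_WeaponBase is a weapon pickup actor, apparently the base for the game's weapons.
; When its sphere overlaps an actor tagged Player, it sends that actor an equip message with itself and stops physics on its skeletal mesh.
; The Interaction event sends a respawn message to the owner, then destroys the weapon.
; Rotation and timeline-driven offset logic is disconnected and never runs, and PickUpRef is an empty stub.
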(event `/Game/Items/Interfaces/BPI_ItemSpawner.Interaction`
  (message `/Game/Items/Interfaces/BPI_ItemSpawner.Respawn` (`self.GetOwner`))
  (`self.K2_DestroyActor`))

(event `self.ReceiveTick`
  (params (DeltaSeconds :type "Float (single-precision)")))

(event `self.Sphere.OnComponentBeginOverlap`
  (params (OverlappedComponent :type "PrimitiveComponent Object Reference") (OtherActor :type "Actor Object Reference") (OtherComp :type "PrimitiveComponent Object Reference") (OtherBodyIndex :type Integer) (bFromSweep :type Boolean) (SweepResult :type "HitResult Structure (by ref)"))
  (if true
    (if (`self.ActorHasTag` OtherActor "Player")
      (message `/Game/Items/Interfaces/INT_PlayerCharacter.EquipWeapon` OtherActor self)
      (`PrimitiveComponent.SetSimulatePhysics` (`self.SkeletalMesh`) false))))

(fn `PickUpRef`
  (returns (PickupRef :type "/Game/Items/WeaponsBaseFolder/BP_Pickup Object Reference"))
  (return null))

(fn `UserConstructionScript`)